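; Trigger volume, a child Blueprint, that opens and closes a referenced BP_Sliding_Door_Y as the player's BP_FPSController overlaps its Box.
; On begin overlap it calls CheckInventoryMessage on the actor with an empty string and, if that returns true, opens the door after OpenDelay.
; On end overlap it closes the door after CloseDelay, without an inventory check.
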(event OnComponentBeginOverlap(Box)
  (params (OverlappedComponent :type Primitive%20Component%20Object%20Reference) (OtherActor :type Actor%20Object%20Reference) (OtherComp :type Primitive%20Component%20Object%20Reference) (OtherBodyIndex :type Integer) (bFromSweep :type Boolean) (SweepResult :type Hit%20Result%20Structure%20%28by%20ref%29))
  ;[1 1 1] Open door on overlap
  (bind _key_picked_up (Class|Inventory|CheckInventory(Message) OtherActor))
  (if _key_picked_up
    (Utilities|Casting|CastToBP_FPSController OtherActor)
    (Utilities|FlowControl|Delay (Variables|Default|GetOpenDelay))
    (bind _asbp_sliding_door_y (Utilities|Casting|CastToBP_Sliding_Door_Y (Variables|Default|GetDoorRef)))
    (Default|OpenDoor _asbp_sliding_door_y)))

(event OnComponentEndOverlap(Box)
  (params (OverlappedComponent :type Primitive%20Component%20Object%20Reference) (OtherActor :type Actor%20Object%20Reference) (OtherComp :type Primitive%20Component%20Object%20Reference) (OtherBodyIndex :type Integer))
  ;[1 1 1] Close door on overlap
  (Utilities|Casting|CastToBP_FPSController OtherActor)
  (Utilities|FlowControl|Delay (Variables|Default|GetCloseDelay))
  (bind _asbp_sliding_door_y (Utilities|Casting|CastToBP_Sliding_Door_Y (Variables|Default|GetDoorRef)))
  (Default|CloseDoor _asbp_sliding_door_y))

(event EventBeginPlay
  (|CallParentFunction) ; This node is disabled and will not be called.\nDrag off pins to build functionality.
)

(event Collision|EventActorBeginOverlap
  (params (OtherActor :type Actor%20Object%20Reference))
  (|CallParentFunction OtherActor) ; This node is disabled and will not be called.\nDrag off pins to build functionality.
)

(fn ConstructionScript
  (|CallParentFunction))