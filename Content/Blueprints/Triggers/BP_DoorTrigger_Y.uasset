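; Door trigger that opens and closes a referenced BP_SlidingDoor_Y for an overlapping BP_FPSController that passes an inventory check.
; Overlap begin and end each call CheckInventoryMessage on the other actor with an empty string, printing an inaccessible message on failure.
; The doorway starts with red glow and turns blue on a passed entry check, before the cast, and never reverts.
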(event EventBeginPlay
  ;[1 1 1] Starts with red glow material
  (Rendering|Material|SetMaterial (Variables|Default|GetDoorway) 0 "/Game/Materials/M_Red_Glow.M_Red_Glow"))

(event Collision|EventActorBeginOverlap
  (params (OtherActor :type Actor%20Object%20Reference))
  ;[1 1 1] Sliding Doors
  (bind _key_picked_up (Class|Inventory|CheckInventory(Message) OtherActor))
  (if _key_picked_up
    (Rendering|Material|SetMaterial (Variables|Default|GetDoorway) 0 "/Game/Materials/M_Blue_Glow.M_Blue_Glow")
    (Utilities|Casting|CastToBP_FPSController OtherActor)
    (bind _asbp_sliding_door_y (Utilities|Casting|CastToBP_SlidingDoor_Y (Variables|Default|GetDoorRef)))
    (Default|OpenDoor _asbp_sliding_door_y)
    (else
      (Development|PrintString "DOOR INACCESSIBLE" true true "(R=0.625000,G=0.000000,B=0.000000,A=1.000000)"))))

(event Collision|EventActorEndOverlap
  (params (OtherActor :type Actor%20Object%20Reference))
  ;[1 1 1] Sliding Doors
  (bind _key_picked_up (Class|Inventory|CheckInventory(Message) OtherActor))
  (if _key_picked_up
    (Utilities|Casting|CastToBP_FPSController OtherActor)
    (bind _asbp_sliding_door_y (Utilities|Casting|CastToBP_SlidingDoor_Y (Variables|Default|GetDoorRef)))
    (Default|CloseDoor _asbp_sliding_door_y)
    (else
      (Development|PrintString "DOOR INACCESSIBLE" true true "(R=0.625000,G=0.000000,B=0.000000,A=1.000000)"))))

(fn ConstructionScript)