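; Base door trigger Blueprint that gates a doorway on an inventory check of the overlapping actor.
; The doorway starts glowing red; a passed CheckInventoryMessage on overlap waits OpenDelay, turns it blue and plays the door sound at world origin.
; End overlap repeats the check and replays the sound after CloseDelay, leaving the material unchanged; failed checks print "DOOR INACCESSIBLE".
; The checked message is empty and no door movement happens here.
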(event EventBeginPlay
  ;[1 1 1] Starts with red glow material
  (Rendering|Material|SetMaterial (Variables|Default|GetDoorway) 0 "/Game/Materials/Glowing/M_Red_Glow.M_Red_Glow"))

(event Collision|EventActorBeginOverlap
  (params (OtherActor :type Actor%20Object%20Reference))
  ;[1 1 1] Sliding Doors
  (bind _key_picked_up (Class|Inventory|CheckInventory(Message) OtherActor))
  (if _key_picked_up
    (Utilities|FlowControl|Delay (Variables|Default|GetOpenDelay))
    (Rendering|Material|SetMaterial (Variables|Default|GetDoorway) 0 "/Game/Materials/Glowing/M_Blue_Glow.M_Blue_Glow")
    (Audio|PlaySoundatLocation "/Game/Sounds/SFX/Door/S_Door_Cue.S_Door_Cue" "0, 0, 0" "0, 0, 0" 1.0 1.0 0.0 0 0 0)
    (else
      (Development|PrintString "DOOR INACCESSIBLE" true true "(R=0.625000,G=0.000000,B=0.000000,A=1.000000)"))))

(event Collision|EventActorEndOverlap
  (params (OtherActor :type Actor%20Object%20Reference))
  ;[1 1 1] Sliding Doors
  (bind _key_picked_up (Class|Inventory|CheckInventory(Message) OtherActor))
  (if _key_picked_up
    (if _key_picked_up
      (Utilities|FlowControl|Delay (Variables|Default|GetCloseDelay))
      (Audio|PlaySoundatLocation "/Game/Sounds/SFX/Door/S_Door_Cue.S_Door_Cue" "0, 0, 0" "0, 0, 0" 1.0 1.0 0.0 0 0 0))
    (else
      (Development|PrintString "DOOR INACCESSIBLE" true true "(R=0.625000,G=0.000000,B=0.000000,A=1.000000)"))))

(fn ConstructionScript)