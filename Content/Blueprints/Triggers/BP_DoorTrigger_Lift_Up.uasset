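; Door trigger for a lift that drives a referenced BP_SlidingDoor_Y and switches the doorway glow between red (initial) and blue.
; Tick polls the player controller's CallLiftUp flag, opening the door while it is set.
; Leaving FrontTrigger clears that flag and closes the door for the player, without resetting the glow.
; BackTrigger opens and closes the door on player overlap after delays, updating the glow.
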(event OnComponentBeginOverlap(BackTrigger)
  (params (OverlappedComponent :type Primitive%20Component%20Object%20Reference) (OtherActor :type Actor%20Object%20Reference) (OtherComp :type Primitive%20Component%20Object%20Reference) (OtherBodyIndex :type Integer) (bFromSweep :type Boolean) (SweepResult :type Hit%20Result%20Structure%20%28by%20ref%29))
  ;[1 1 1] Open Door
  (Utilities|Casting|CastToBP_FPSController OtherActor)
  (if true
    (bind _asbp_sliding_door_y (Utilities|Casting|CastToBP_SlidingDoor_Y (Variables|Default|GetDoorRef)))
    (Utilities|FlowControl|Delay (Variables|Default|GetOpenDelay))
    (Default|OpenDoor _asbp_sliding_door_y)
    (Rendering|Material|SetMaterial (Variables|Default|GetDoorway) 0 "/Game/Materials/M_Blue_Glow.M_Blue_Glow")))

(event OnComponentEndOverlap(BackTrigger)
  (params (OverlappedComponent :type Primitive%20Component%20Object%20Reference) (OtherActor :type Actor%20Object%20Reference) (OtherComp :type Primitive%20Component%20Object%20Reference) (OtherBodyIndex :type Integer))
  ;[1 1 1] Close Door
  (Utilities|Casting|CastToBP_FPSController OtherActor)
  (if true
    (bind _asbp_sliding_door_y (Utilities|Casting|CastToBP_SlidingDoor_Y (Variables|Default|GetDoorRef)))
    (Utilities|FlowControl|Delay (Variables|Default|GetCloseDelay))
    (Default|CloseDoor _asbp_sliding_door_y)
    (Utilities|FlowControl|Delay 2.0)
    (Rendering|Material|SetMaterial (Variables|Default|GetDoorway) 0 "/Game/Materials/M_Red_Glow.M_Red_Glow")))

(event OnComponentBeginOverlap(FrontTrigger)
  (params (OverlappedComponent :type Primitive%20Component%20Object%20Reference) (OtherActor :type Actor%20Object%20Reference) (OtherComp :type Primitive%20Component%20Object%20Reference) (OtherBodyIndex :type Integer) (bFromSweep :type Boolean) (SweepResult :type Hit%20Result%20Structure%20%28by%20ref%29))
  ;[1 1 1] Sliding Doors
)

(event OnComponentEndOverlap(FrontTrigger)
  (params (OverlappedComponent :type Primitive%20Component%20Object%20Reference) (OtherActor :type Actor%20Object%20Reference) (OtherComp :type Primitive%20Component%20Object%20Reference) (OtherBodyIndex :type Integer))
  ;[1 1 1] Sliding Doors
  (Variables|/Game/Blueprints/BP_FPSController.BP_FPSController_C|SetCallLiftUp (stale EventTick _asbp_fpscontroller) false)
  (if true
    (Utilities|Casting|CastToBP_FPSController OtherActor)
    (bind _asbp_sliding_door_y (Utilities|Casting|CastToBP_SlidingDoor_Y (Variables|Default|GetDoorRef)))
    (Default|CloseDoor _asbp_sliding_door_y)))

(event EventBeginPlay
  ;[1 1 1] Starts with red glow material
  (Rendering|Material|SetMaterial (Variables|Default|GetDoorway) 0 "/Game/Materials/M_Red_Glow.M_Red_Glow"))

(event EventTick
  (params (DeltaSeconds :type Float%20%28single-precision%29))
  ;[1 1 1] Sliding Doors
  (bind _asbp_fpscontroller (Utilities|Casting|CastToBP_FPSController (Game|GetPlayerCharacter 0)))
  (if (Variables|/Game/Blueprints/BP_FPSController.BP_FPSController_C|GetCallLiftUp _asbp_fpscontroller)
    (Rendering|Material|SetMaterial (Variables|Default|GetDoorway) 0 "/Game/Materials/M_Blue_Glow.M_Blue_Glow")
    (bind _asbp_sliding_door_y (Utilities|Casting|CastToBP_SlidingDoor_Y (Variables|Default|GetDoorRef)))
    (Default|OpenDoor _asbp_sliding_door_y)))

(fn ConstructionScript)