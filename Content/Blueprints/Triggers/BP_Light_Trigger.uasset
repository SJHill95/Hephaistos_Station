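; Trigger actor that switches up to four referenced BP_Light actors on when a BP_FPSController overlaps it and off when that overlap ends.
; Each event runs a four-branch Sequence, giving every light slot its own on and off delay for staggered switching.
; Each reference is cast to BP_Light after its delay, then TurnLightOn or TurnLightOff is called.
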(event Collision|EventActorBeginOverlap
  (params (OtherActor :type Actor%20Object%20Reference))
  ;[1 1 1] Turn on lights
  (Utilities|Casting|CastToBP_FPSController OtherActor)
  (Utilities|FlowControl|Sequence
    (:then_0
      (Utilities|FlowControl|Delay (Variables|Default|GetLight01%20OnDelay))
      (bind _asbp_light (Utilities|Casting|CastToBP_Light (Variables|Default|GetLightRef01)))
      (Default|TurnLighton _asbp_light))
    (:then_1
      (Utilities|FlowControl|Delay (Variables|Default|GetLight02%20OnDelay))
      (bind _asbp_light_2 (Utilities|Casting|CastToBP_Light (Variables|Default|GetLightRef02)))
      (Default|TurnLighton _asbp_light_2))
    (:then_2
      (Utilities|FlowControl|Delay (Variables|Default|GetLight03%20OnDelay))
      (bind _asbp_light_3 (Utilities|Casting|CastToBP_Light (Variables|Default|GetLightRef03)))
      (Default|TurnLighton _asbp_light_3))
    (:then_3
      (Utilities|FlowControl|Delay (Variables|Default|GetLight04%20OnDelay))
      (bind _asbp_light_4 (Utilities|Casting|CastToBP_Light (Variables|Default|GetLightRef04)))
      (Default|TurnLighton _asbp_light_4))))

(event Collision|EventActorEndOverlap
  (params (OtherActor :type Actor%20Object%20Reference))
  ;[1 1 1] Turn off lights
  (Utilities|Casting|CastToBP_FPSController OtherActor)
  (Utilities|FlowControl|Sequence
    (:then_0
      (Utilities|FlowControl|Delay (Variables|Default|GetLight%2001%20OffDelay))
      (bind _asbp_light (Utilities|Casting|CastToBP_Light (Variables|Default|GetLightRef01)))
      (Default|TurnLightOff _asbp_light))
    (:then_1
      (Utilities|FlowControl|Delay (Variables|Default|GetLight%2002%20OffDelay))
      (bind _asbp_light_2 (Utilities|Casting|CastToBP_Light (Variables|Default|GetLightRef02)))
      (Default|TurnLightOff _asbp_light_2))
    (:then_2
      (Utilities|FlowControl|Delay (Variables|Default|GetLight%2003%20OffDelay))
      (bind _asbp_light_3 (Utilities|Casting|CastToBP_Light (Variables|Default|GetLightRef03)))
      (Default|TurnLightOff _asbp_light_3))
    (:then_3
      (Utilities|FlowControl|Delay (Variables|Default|GetLight%2004%20OffDelay))
      (bind _asbp_light_4 (Utilities|Casting|CastToBP_Light (Variables|Default|GetLightRef04)))
      (Default|TurnLightOff _asbp_light_4))))

(fn ConstructionScript)