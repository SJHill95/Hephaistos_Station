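; BP_Sliding_Door_Y is a sliding door that moves along the world Y axis through its OpenDoor and CloseDoor events.
; BeginPlay caches the Door component's world location as the closed position.
; A timeline lerps the whole actor from that position to an absolute YLocation, keeping X and Z fixed, without sweeping.
; CloseDoor reverses the same timeline.
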(event Custom|Close%20Door
  (bind _worldloc (Variables|Default|GetWorldLoc))
  ;[1 1 1] Door Movement
  (bind _newtrack_0 (Timeline|Timeline_0 Reverse)
    (:Update
      (Transformation|SetActorLocation (Math|Vector|Lerp(Vector) (Variables|Default|GetWorldLoc) (Math|Vector|MakeVector (.x _worldloc) (Variables|Default|GetY%20Location) (.z _worldloc)) _newtrack_0) false false))))

(event Custom|Open%20Door
  (bind _worldloc (Variables|Default|GetWorldLoc))
  ;[1 1 1] Door Movement
  (bind _newtrack_0 (Timeline|Timeline_0 Play)
    (:Update
      (Transformation|SetActorLocation (Math|Vector|Lerp(Vector) (Variables|Default|GetWorldLoc) (Math|Vector|MakeVector (.x _worldloc) (Variables|Default|GetY%20Location) (.z _worldloc)) _newtrack_0) false false))))

(event EventBeginPlay
  ;[1 1 1] Gets doors world location
  (Variables|Default|SetWorldLoc (Transformation|GetWorldLocation (Variables|Default|GetDoor))))

(fn ConstructionScript)