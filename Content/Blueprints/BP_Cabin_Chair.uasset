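; BP_Cabin_Chair is an interactable chair that the player can sit in and leave.
; Interact alternates via FlipFlop, disabling or restoring movement on the player's BP_FPSController.
; Sitting plays a timeline that lerps the spring arm to a seated offset while pinning the character at SitLocation.
; Exiting moves the character to the Plane component's location without resetting the spring arm.
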(event EventInteract
  ;[1 1 1] Sit in chair
  (Utilities|FlowControl|FlipFlop
    (:A
      (bind _asbp_fpscontroller (Utilities|Casting|CastToBP_FPSController (Game|GetPlayerCharacter 0)))
      (Variables|/Game/Blueprints/BP_FPSController.BP_FPSController_C|SetMovementDisabled _asbp_fpscontroller true)
      (Components|Activation|ToggleActive (Variables|/Script/Engine.Character|GetCharacterMovement _asbp_fpscontroller))
      (bind _newtrack_0 (Timeline|Timeline_0 Play)
        (:Update
          (Transformation|SetRelativeLocation (Variables|/Game/Blueprints/BP_FPSController.BP_FPSController_C|GetSpringArm _asbp_fpscontroller) (Math|Vector|Lerp(Vector) (Variables|/Script/Engine.SceneComponent|GetRelativeLocation (Variables|/Game/Blueprints/BP_FPSController.BP_FPSController_C|GetSpringArm _asbp_fpscontroller)) "0, 0,50.000000" _newtrack_0) false false)
          (Transformation|SetActorLocation _asbp_fpscontroller (Transformation|GetWorldLocation (Variables|Default|GetSit_Location)) false false))))
    (:B
      ;[1 1 1] Exit chair
      (bind _asbp_fpscontroller_2 (Utilities|Casting|CastToBP_FPSController (Game|GetPlayerCharacter 0)))
      (Variables|/Game/Blueprints/BP_FPSController.BP_FPSController_C|SetMovementDisabled _asbp_fpscontroller_2 false)
      (Components|Activation|ToggleActive (Variables|/Script/Engine.Character|GetCharacterMovement _asbp_fpscontroller_2))
      (Transformation|SetActorLocation _asbp_fpscontroller_2 (Transformation|GetWorldLocation (Variables|Default|GetPlane)) false false))))

(fn ConstructionScript)