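; Interactable lift keypad button that calls the lift downward.
; On interaction it sets the CallLift and CallLiftDown flags on the player's BP_FPSController and prints the flag for debugging.
; Every tick it casts to that controller again and swaps the mesh material between green and red to reflect whether a downward call is active.
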(event EventInteract
  ;[1 1 1] Call Lift
  (bind _asbp_fpscontroller (Utilities|Casting|CastToBP_FPSController (Game|GetPlayerCharacter 0)))
  (Variables|/Game/Blueprints/BP_FPSController.BP_FPSController_C|SetCallLift _asbp_fpscontroller true)
  (bind _output_get (Variables|/Game/Blueprints/BP_FPSController.BP_FPSController_C|SetCallLiftDown _asbp_fpscontroller true))
  (Development|PrintString (Utilities|String|ToString(Boolean) _output_get)))

(event EventTick
  (params (DeltaSeconds :type Float%20%28single-precision%29))
  ;[1 1 1] Change Material
  (bind _asbp_fpscontroller (Utilities|Casting|CastToBP_FPSController (Game|GetPlayerCharacter 0)))
  (if (Variables|/Game/Blueprints/BP_FPSController.BP_FPSController_C|GetCallLiftDown _asbp_fpscontroller)
    (Rendering|Material|SetMaterial (Variables|Default|GetStaticMesh) 0 "/Game/Materials/M_Lift_Button_Green.M_Lift_Button_Green")
    (else
      (Rendering|Material|SetMaterial (Variables|Default|GetStaticMesh) 0 "/Game/Materials/M_Lift_Button_Red.M_Lift_Button_Red"))))

(fn ConstructionScript)