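; Interactable keypad for calling the lift in the up direction.
; On Interact it sets the CallLift and CallLiftUp flags on the player's BP_FPSController and plays a call sound at the world origin.
; Every Tick it casts the player character again and reads CallLiftUp to switch the screen material between green and red, so the lift call state lives on the player character.
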(event EventInteract
  ;[1 1 1] Call Lift
  (bind _asbp_fpscontroller (Utilities|Casting|CastToBP_FPSController (Game|GetPlayerCharacter 0)))
  (Variables|/Game/Blueprints/BP_FPSController.BP_FPSController_C|SetCallLift _asbp_fpscontroller true)
  (Variables|/Game/Blueprints/BP_FPSController.BP_FPSController_C|SetCallLiftUp _asbp_fpscontroller true)
  (Audio|PlaySoundatLocation "/Game/Sounds/SFX/S_CallLift_Cue.S_CallLift_Cue" "0, 0, 0" "0, 0, 0" 1.0 1.0 0.0 0 0 0))

(event EventTick
  (params (DeltaSeconds :type Float%20%28single-precision%29))
  ;[1 1 1] Change Material
  (bind _asbp_fpscontroller (Utilities|Casting|CastToBP_FPSController (Game|GetPlayerCharacter 0)))
  (if (Variables|/Game/Blueprints/BP_FPSController.BP_FPSController_C|GetCallLiftUp _asbp_fpscontroller)
    (Rendering|Material|SetMaterial (Variables|Default|GetScreen) 0 "/Game/Materials/M_Lift_Button_Green.M_Lift_Button_Green")
    (else
      (Rendering|Material|SetMaterial (Variables|Default|GetScreen) 0 "/Game/Materials/M_Lift_Button_Red.M_Lift_Button_Red"))))

(fn ConstructionScript)