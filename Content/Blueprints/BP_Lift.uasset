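; BP_Lift is an elevator actor that moves vertically when a BP_FPSController overlaps it with CallLift set.
; BeginPlay stores the Lift component's world location as the starting point.
; Qualifying overlaps alternate through a FlipFlop between playing and reversing a timeline, each after its own delay.
; The timeline lerps the actor's location from that start to a hard-coded world height, keeping X and Y.
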(event EventBeginPlay
  ;[1 1 1] Gets lifts world location
  (Variables|Default|SetWorldLoc (Transformation|GetWorldLocation (Variables|Default|GetLift))))

(event Collision|EventActorBeginOverlap
  (params (OtherActor :type Actor%20Object%20Reference))
  (bind _worldloc (Variables|Default|GetWorldLoc))
  ;[1 1 1] Lift Movement
  (bind _asbp_fpscontroller (Utilities|Casting|CastToBP_FPSController OtherActor))
  (if (Variables|/Game/Characters/BP_FPSController.BP_FPSController_C|GetCallLift _asbp_fpscontroller)
    (Utilities|FlowControl|FlipFlop
      (:A
        (Utilities|FlowControl|Delay (Variables|Default|GetUpDelay))
        (bind _newtrack_1 (Timeline|Timeline_0 Play)
          (:Update
            (Transformation|SetActorLocation (Math|Vector|Lerp(Vector) (Variables|Default|GetWorldLoc) (Math|Vector|MakeVector (.x _worldloc) (.y _worldloc) 2.7e+02) _newtrack_1) false false))))
      (:B
        (Utilities|FlowControl|Delay (Variables|Default|GetDownDelay))
        (Timeline|Timeline_0 Reverse)))))

(fn ConstructionScript)