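; First-person player character handling movement, sprint, timeline-eased crouch, timed footstep sounds and a key inventory.
; Short camera line traces drive physics-handle pickup, send interact messages to hit actors and feed a hit flag to the HUD each tick.
; Held objects follow a pickup location component through the physics handle.
; It also creates the HUD and pause menu widgets, toggling pause and input mode on input.
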(event Custom|PlayFootstepSound
  ;[1 1 1] Footsteps
  (Audio|PlaySoundatLocation "/Game/Sounds/SFX/Footsteps/S_Footsteps_Cue.S_FootSteps_Cue" (- (Transformation|GetActorLocation) "0, 0,10.000000") "0, 0, 0" 1.0 1.0 0.0 0 0 0))

(event EventAddInventory
  (params (Key :type String))
  ;[1 1 1] Adds key to inventory
  (Utilities|Array|Add (Variables|Default|GetInventory) Key)
  (Development|PrintString "key added to inventory"))

(event EventBeginPlay
  ;[1 1 1] Add HUD & Pause to viewport
  (bind _returnvalue (UserInterface|CreateWidget "/Game/UI/HUD.HUD_C"))
  (bind _output_get (Variables|Default|SetHUD _returnvalue))
  (UserInterface|Viewport|AddtoViewport _output_get 0)
  (bind _returnvalue_2 (UserInterface|CreateWidget "/Game/UI/WB_Pause_Menu.WB_Pause_Menu_C"))
  (bind _output_get_2 (Variables|Default|SetPauseMenu _returnvalue_2))
  (UserInterface|Viewport|AddtoViewport _output_get_2 0)
  (Widget|SetVisibility (Variables|Default|GetPauseMenu) "Hidden"))

(event EventTick
  (params (DeltaSeconds :type Float%20%28single-precision%29))
  (bind _firstpersoncamera (Variables|Default|GetFirstPersonCamera))
  (bind _returnvalue (Transformation|GetWorldLocation _firstpersoncamera))
  ;[1 1 1] Raycast display widget
  (Physics|Components|PhysicsHandle|SetTargetLocation (Variables|Default|GetPhysicsHandle) (Transformation|GetWorldLocation (Variables|Default|GetPickup_Item_Location)))
  (bind _outhit (Collision|LineTraceByChannel _returnvalue (+ _returnvalue (* (Math|Vector|GetForwardVector (Transformation|GetWorldRotation _firstpersoncamera)) 2e+02)) "TraceTypeQuery3" false 0 "None"))
  (Variables|/Game/UI/HUD.HUD_C|SetLineTraceHit (Variables|Default|GetHUD) (.bBlockingHit (Collision|BreakHitResult _outhit))))

(event Input|ActionEvents|InputActionPause
  (params (Key :type Key%20Structure :default "None"))
  ;[1 1 1] Pause Game
  (:Pressed
    (if (Variables|Default|GetPause)
      (Input|SetInputModeGameOnly (Game|GetPlayerController 0))
      (Widget|SetVisibility (Variables|Default|GetPauseMenu) "Hidden")
      (Game|SetGamePaused false)
      (Variables|Default|SetPause false)
      (else
        (Widget|SetVisibility (Variables|Default|GetPauseMenu) "Visible")
        (Game|SetGamePaused true)
        (Input|SetInputModeGameandUI (Game|GetPlayerController 0) (Variables|Default|GetPauseMenu) "DoNotLock" true)
        (Variables|Default|SetPause true)))))

(event Input|ActionEvents|InputActionCrouch
  (params (Key :type Key%20Structure :default "None"))
  (bind _charactermovement (Variables|Character|GetCharacterMovement))
  ;[1 1 1] Crouch Controls
  (:Pressed
    (if (not (Variables|Default|GetMovementDisabled))
      (Variables|/Script/Engine.CharacterMovementComponent|SetMaxWalkSpeed _charactermovement 2e+02)
      (bind _newtrack_0 (Timeline|CrouchTimeLine PlayFromStart)
        (:Update
          (Transformation|SetRelativeLocation (Variables|Default|GetSpringArm) (Math|Vector|Lerp(Vector) (Variables|/Script/Engine.SceneComponent|GetRelativeLocation (Variables|Default|GetSpringArm)) "0, 0,20.000000" _newtrack_0) false false)))))
  (:Released
    (if (not (Variables|Default|GetMovementDisabled))
      (Variables|/Script/Engine.CharacterMovementComponent|SetMaxWalkSpeed _charactermovement 4e+02)
      (bind _newtrack_0_2 (Timeline|Timeline_0 PlayFromStart)
        (:Update
          (Transformation|SetRelativeLocation (Variables|Default|GetSpringArm) (Math|Vector|Lerp(Vector) (Variables|/Script/Engine.SceneComponent|GetRelativeLocation (Variables|Default|GetSpringArm)) "0, 0,50.000000" _newtrack_0_2) false false))))))

(event Input|ActionEvents|InputActionSprint
  (params (Key :type Key%20Structure :default "None"))
  (bind _charactermovement (Variables|Character|GetCharacterMovement))
  ;[1 1 1] Sprint Controls
  (:Pressed
    (Variables|/Script/Engine.CharacterMovementComponent|SetMaxWalkSpeed _charactermovement 8e+02)
    (Variables|Default|SetFootstepTime 0.4))
  (:Released
    (Variables|/Script/Engine.CharacterMovementComponent|SetMaxWalkSpeed _charactermovement 4e+02)
    (Variables|Default|SetFootstepTime 0.5)))

(event Input|ActionEvents|InputActionJump
  (params (Key :type Key%20Structure :default "None"))
  ;[1 1 1] Jump Controls
  (:Pressed
    (Character|Jump))
  (:Released
    (Character|StopJumping)))

(event Input|ActionEvents|InputActionAction
  (params (Key :type Key%20Structure :default "None"))
  (bind _firstpersoncamera (Variables|Default|GetFirstPersonCamera))
  (bind _returnvalue (Transformation|GetWorldLocation _firstpersoncamera))
  ;[1 1 1] Ray Cast Interaction
  (:Pressed
    (bind (_outhit _returnvalue_2) (Collision|LineTraceByChannel _returnvalue (+ _returnvalue (* (Math|Vector|GetForwardVector (Transformation|GetWorldRotation _firstpersoncamera)) 2e+02)) "TraceTypeQuery1" false 0 "None"))
    (if _returnvalue_2
      (Class|InteractionInterface|Interact(Message) (.HitActor (Collision|BreakHitResult _outhit))))))

(event Input|ActionEvents|InputActionPickup
  (params (Key :type Key%20Structure :default "None"))
  (bind _firstpersoncamera (Variables|Default|GetFirstPersonCamera))
  (bind _returnvalue (Transformation|GetWorldLocation _firstpersoncamera))
  ;[1 1 1] Ray Cast Grabber
  (:Pressed
    (bind (_outhit _returnvalue_2) (Collision|LineTraceByChannel _returnvalue (+ _returnvalue (* (Math|Vector|GetForwardVector (Transformation|GetWorldRotation _firstpersoncamera)) 2e+02)) "TraceTypeQuery1" false 0 "None"))
    (if _returnvalue_2
      (if (Physics|IsSimulatingPhysics (.HitComponent (Collision|BreakHitResult _outhit)) "None")
        (Class|PhysicsHandleComponent|GrabComponentatLocation (Variables|Default|GetPhysicsHandle) (.HitComponent (Collision|BreakHitResult _outhit)) "None" (Transformation|GetWorldLocation (.HitComponent (Collision|BreakHitResult _outhit)))))))
  (:Released
    (Physics|Components|PhysicsHandle|ReleaseComponent (Variables|Default|GetPhysicsHandle))))

(event Input|AxisEvents|InputAxisMouse-Look-Left-Right
  (params (AxisValue :type Float%20%28single-precision%29))
  ;[1 1 1] Mouse Controls
  (Pawn|Input|AddControllerYawInput AxisValue))

(event Input|AxisEvents|InputAxisMouse-Look-Up-Down
  (params (AxisValue :type Float%20%28single-precision%29))
  ;[1 1 1] Mouse Controls
  (Pawn|Input|AddControllerPitchInput AxisValue))

(event Input|AxisEvents|InputAxisForward-Backward
  (params (AxisValue :type Float%20%28single-precision%29))
  (bind _returnvalue (Transformation|GetVelocity))
  ;[1 1 1] WASD Controls
  (Pawn|Input|AddMovementInput (Math|Vector|GetForwardVector (Math|Rotator|MakeRotator 0.0 0.0 (.yaw (Pawn|GetControlRotation :!class /Script/Engine.Pawn)))) AxisValue false)
  ;[1 1 1] Footsteps
  (if (and (Math|Boolean|ORBoolean (> (.x _returnvalue) 2.0) (< (.x _returnvalue) -2.0) (> (.y _returnvalue) 2.0) (< (.y _returnvalue) -2.0)) (== (.z _returnvalue) 0.0))
    (Utilities|FlowControl|DoOnce false :!label _label
      (:Completed
        (bind _returnvalue_2 (Utilities|Time|SetTimerbyEvent (delegate Custom|PlayFootstepSound) (Variables|Default|GetFootstepTime) true))))
    (else
      (Utilities|Time|ClearandInvalidateTimerbyHandle _returnvalue_2)
      (goto _label Reset))))

(event Input|AxisEvents|InputAxisLeft-Right
  (params (AxisValue :type Float%20%28single-precision%29))
  (bind _returnvalue (Transformation|GetVelocity))
  ;[1 1 1] WASD Controls
  (Pawn|Input|AddMovementInput (Math|Vector|GetRightVector (Math|Rotator|MakeRotator 0.0 0.0 (.yaw (Pawn|GetControlRotation :!class /Script/Engine.Pawn)))) AxisValue false)
  ;[1 1 1] Footsteps
  (if (and (Math|Boolean|ORBoolean (> (.x _returnvalue) 2.0) (< (.x _returnvalue) -2.0) (> (.y _returnvalue) 2.0) (< (.y _returnvalue) -2.0)) (== (.z _returnvalue) 0.0))
    (Utilities|FlowControl|DoOnce false :!label _label
      (:Completed
        (bind _returnvalue_2 (Utilities|Time|SetTimerbyEvent (delegate Custom|PlayFootstepSound) (Variables|Default|GetFootstepTime) true))))
    (else
      (Utilities|Time|ClearandInvalidateTimerbyHandle _returnvalue_2)
      (goto _label Reset))))

(fn ConstructionScript)

(fn CheckInventory
  (params (Key :type String))
  (return (Utilities|Array|ContainsItem (Variables|Default|GetInventory) Key)))